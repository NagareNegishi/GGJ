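; BP_Tree is a wandering pickup that the player and BP_Taka can take, updating the bullet-hell game mode's score.
; Each tick it moves with sweep along a random, unnormalized XY direction, re-rolled whenever its mesh hits anything else.
; A player hit calls Fat on the player.
; Taken then passes who took it to UpdateScore, plays that taker's impact sound and destroys the tree.
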(event `self.ReceiveBeginPlay`
  (`self.GenerateDirection`))

(event `self.ReceiveActorBeginOverlap`
  (params (OtherActor :type "Actor Object Reference")))

(event `self.ReceiveTick`
  (params (DeltaSeconds :type "Float (single-precision)"))
  (`self.K2_SetActorLocation` (+ (* DeltaSeconds (`self.Speed`) (`self.Direction`)) (`self.K2_GetActorLocation`)) true))

(event `self.StaticMesh.OnComponentHit`
  (params (HitComponent :type "PrimitiveComponent Object Reference") (OtherActor :type "Actor Object Reference") (OtherComp :type "PrimitiveComponent Object Reference") (NormalImpulse :type "Vector Structure") (Hit :type "HitResult Structure (by ref)"))
  (bind _asbp_player (cast `/Game/BluePrint/Player/BP_Player` OtherActor)
    (:`then`
      (`/Game/BluePrint/Player/BP_Player.Fat` _asbp_player)
      (`self.Taken` true))
    (:`CastFailed`
      (cast `/Game/BluePrint/Enemies/BP_Taka` OtherActor
        (:`then`
          (`self.Taken` false))
        (:`CastFailed`
          (`self.GenerateDirection`))))))

(fn `GenerateDirection`
  (set `self.Direction` (`KismetMathLibrary.MakeVector` (`KismetMathLibrary.RandomFloatInRange` -1.0 1.0) (`KismetMathLibrary.RandomFloatInRange` -1.0 1.0))))

(fn `Taken`
  (params (isPlayer :type Boolean))
  (if isPlayer
    (bind _asbp_bullet_hell_game_mode (cast `/Game/BluePrint/BP_BulletHellGameMode` (`GameplayStatics.GetGameMode`)))
    (`/Game/BluePrint/BP_BulletHellGameMode.UpdateScore` _asbp_bullet_hell_game_mode true)
    (`GameplayStatics.PlaySound2D` (`self.Impact Sound`) 1.0 1.0 0.0 null null)
    (else
      (bind _asbp_bullet_hell_game_mode_2 (cast `/Game/BluePrint/BP_BulletHellGameMode` (`GameplayStatics.GetGameMode`)))
      (`/Game/BluePrint/BP_BulletHellGameMode.UpdateScore` _asbp_bullet_hell_game_mode_2 false)
      (`GameplayStatics.PlaySound2D` (`self.Impact Sound_taka`) 1.0 1.0 0.0 null null)))
  (`self.K2_DestroyActor`))

(fn `UserConstructionScript`)