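; Base 2D flipbook projectile for player or enemy side, with optional aiming or homing at a target and a periodically randomized sprite scale.
; BeginPlay sets the collision profile by side and ignores the owner.
; On hit, TypeCheck applies side-dependent effects to players, Taka, opposing bullets and ZZZ pickups, then the projectile plays impact effects and destroys itself.
; A reflect branch that turns it into an enemy bullet is left unconnected.
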(event `randomSize`
  ;[1 1 1] changing size here
  (`self.ChangeSize`))

(event `self.ReceiveBeginPlay`
  ;[1 1 1] changing size here
  (`KismetSystemLibrary.K2_SetTimerDelegate` (delegate `randomSize`) 0.5 true)
  (`PrimitiveComponent.IgnoreActorWhenMoving` (`self.Box`) (`self.GetOwner`) true)
  (if (`self.IsPlayerSide`)
    (`PrimitiveComponent.SetCollisionProfileName` (`self.Box`) "PlayerPreSet" true)
    (else
      (`PrimitiveComponent.SetCollisionProfileName` (`self.Box`) "EnemyPreSet" true)))
  (`self.Target`
    (:`then`
      (`self.Rotate to Enemy`))
    (:`else`)))

(event `Rotate to Enemy`
  (set `MovementComponent.Velocity` (* (`KismetMathLibrary.GetDirectionUnitVector` (`self.K2_GetActorLocation`) (`self.K2_GetActorLocation` (`self.Target`))) (`self.Speed`)) (`self.ProjectileMovement`)))

(event `self.Box.OnComponentHit`
  (params (HitComponent :type "PrimitiveComponent Object Reference") (OtherActor :type "Actor Object Reference") (OtherComp :type "PrimitiveComponent Object Reference") (NormalImpulse :type "Vector Structure") (Hit :type "HitResult Structure (by ref)"))
  (bind (_bblockinghit _binitialoverlap _time _distance _location _impactpoint _normal) (`GameplayStatics.BreakHitResult` Hit))
  (`self.OnProjectileHit` OtherActor Hit)
  (bind _name (`self.TypeCheck` OtherActor))
  (switch `string` _name
    (:`Default`
      _)
    (:`Hit`
      _)
    (:`Wall`)
    (:`ZZZ`
      _))
  (bind _returnvalue (`GameplayStatics.SpawnEmitterAtLocation` (`self.Impact Effect`) _location))
  (`ParticleSystemComponent.EndTrails` _returnvalue)
  (`GameplayStatics.PlaySoundAtLocation` (`self.Impact Sound`) _location (struct) 1.0 1.0 0.0 null null null null)
  (`self.K2_DestroyActor`))

(fn `ChangeSize`
  (bind _returnvalue (`KismetMathLibrary.RandomFloatInRange` 0.1 0.3))
  (`SceneComponent.SetRelativeScale3D` (`self.PaperFlipbook`) (`KismetMathLibrary.MakeVector` _returnvalue 0.3 _returnvalue)))

(fn `GenerateDirection`
  (set `self.Direction` (`KismetMathLibrary.MakeVector` (`KismetMathLibrary.RandomFloatInRange` -1.0 1.0) (`KismetMathLibrary.RandomFloatInRange` -1.0 1.0))))

(fn `TypeCheck`
  (params (other :type "Actor Object Reference"))
  (returns (Name :type String))
  (bind _isplayerside (`self.IsPlayerSide`))
  (bind _asbp_player (cast `/Game/BluePrint/Player/BP_Player` other)
    (:`then`
      (if (`self.IsPlayerSide`)
        (return "Player")
        (else
          (`/Game/BluePrint/Player/BP_Player.Wait` _asbp_player)
          (return "Hit"))))
    (:`CastFailed`
      (bind _asbp_projectile_bullet (cast `/Game/BluePrint/Projectiles/BP_Projectile_Bullet` other)
        (:`then`
          (if (`/Game/BluePrint/Projectiles/BP_Projectile_Base.IsPlayerSide` _asbp_projectile_bullet)
            (if (`self.IsPlayerSide`)
              (return "PlayerB")
              (else
                _))
            (elif (`self.IsPlayerSide`)
              _
              (else
                (return "EnemyB"))))
          (`self.K2_DestroyActor` _asbp_projectile_bullet)
          (return "Hit"))
        (:`CastFailed`
          (cast `/Game/BluePrint/Stage/BP_Wall` other
            (:`then`
              (return "Wall"))
            (:`CastFailed`
              (bind _asbp_zzz (cast `/Game/BluePrint/Items/BP_ZZZ` other)
                (:`then`
                  (`/Game/BluePrint/Items/BP_RoamingObject.Taken` _asbp_zzz _isplayerside)
                  (if _isplayerside
                    (bind _asbp_player_2 (cast `/Game/BluePrint/Player/BP_Player` (`GameplayStatics.GetPlayerCharacter` 0))
                      (:`then`
                        (`/Game/BluePrint/Player/BP_Player.Fat` _asbp_player_2))
                      (:`CastFailed`
                        _)))
                  (return "ZZZ"))
                (:`CastFailed`
                  (bind _asbp_taka (cast `/Game/BluePrint/Enemies/BP_Taka` other))
                  (if (`self.IsPlayerSide`)
                    (`/Game/BluePrint/Enemies/BP_Taka.Wait` _asbp_taka)
                    (return "Hit")
                    (else
                      (return "Ignore"))))))))))))

(fn `UserConstructionScript`
  (bind _projectilemovement (`self.ProjectileMovement`))
  (set `ProjectileMovementComponent.InitialSpeed` (`self.Speed`) _projectilemovement)
  (set `ProjectileMovementComponent.MaxSpeed` (`self.Speed`) _projectilemovement)
  (set `ProjectileMovementComponent.ProjectileGravityScale` (`self.Gravity`) _projectilemovement)
  (`self.Target`
    (:`then`
      (if (`self.Is Homing`)
        (set `ProjectileMovementComponent.bIsHomingProjectile` true _projectilemovement)
        (set `ProjectileMovementComponent.HomingTargetComponent` (`Actor.RootComponent` (`self.Target`)) _projectilemovement)))
    (:`else`)))